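; Development child of the Anthem character that adds a debug HUD and flight-path visualization.
; BeginPlay runs the parent logic, puts a DevHUD widget on the viewport and, if IsDebugging is set, starts DrawDebugPath.
; That event re-calls itself after a short delay, leaving timed trails while Flying: a sphere low on the capsule, with red velocity and blue FlyDirection arrows.
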(event Custom|DrawDebugPath
  (bind _capsulecomponent (Variables|Default|GetCapsuleComponent))
  (bind _returnvalue (Transformation|GetWorldLocation _capsulecomponent))
  (bind _returnvalue_2 (Class|CapsuleComponent|GetScaledCapsuleHalfHeightWithoutHemisphere _capsulecomponent))
  (bind _returnvalue_3 (- (.z _returnvalue) _returnvalue_2))
  (bind _returnvalue_4 (Math|Vector|MakeVector (.x _returnvalue) (.y _returnvalue) _returnvalue_3))
  ;[1 1 1] Flying Debug
  (if (Utilities|Enum|Equal(Enum) (Variables|/Script/Engine.CharacterMovementComponent|GetMovementMode (Variables|Character|GetCharacterMovement)) "MOVE_Flying")
    (Rendering|Debug|DrawDebugSphere _returnvalue_4 (Components|Capsule|GetScaledCapsuleRadius _capsulecomponent) 12 "(R=1.000000,G=1.000000,B=1.000000,A=1.000000)" 15.0)
    (Rendering|Debug|DrawDebugArrow _returnvalue_4 (+ _returnvalue_4 (* (Math|Vector|Normalize (Variables|/Script/Engine.MovementComponent|GetVelocity (Variables|Character|GetCharacterMovement))) 1e+02)) 2.0 "(R=1.000000,G=0.000000,B=0.000000,A=1.000000)" 15.0 0.0)
    (Rendering|Debug|DrawDebugArrow _returnvalue_4 (+ _returnvalue_4 (* (Math|Vector|GetForwardVector (Variables|Default|GetflyDirection)) 1e+02)) 2.0 "(R=0.000000,G=0.000000,B=1.000000,A=1.000000)" 15.0 0.0))
  (Utilities|FlowControl|Delay 0.3)
  (CallFunction|DrawDebugPath))

(event EventBeginPlay
  (|CallParentFunction)
  (bind _returnvalue (UserInterface|CreateWidget "/Game/Anthem/Characters/DevHUD.DevHUD_C"))
  (UserInterface|Viewport|AddtoViewport _returnvalue 0)
  (if (Variables|Default|GetbIsDebugging)
    (CallFunction|DrawDebugPath)))

(event Collision|EventActorBeginOverlap
  (params (OtherActor :type Actor%20Object%20Reference)))

(event EventTick
  (params (DeltaSeconds :type Float%20%28single-precision%29))
  (|CallParentFunction DeltaSeconds))

(fn ConstructionScript
  (|CallParentFunction))