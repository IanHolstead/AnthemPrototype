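; BP_AnthemGameMode is the Anthem game mode that handles pausing and resuming the game.
; Pause creates and stores a PauseMenu widget, adds it to the viewport, switches the first player to UI-only input with cursor and click events, and pauses the game.
; UnPause removes the stored widget, restores game-only input, hides the cursor, disables click events and unpauses.
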(event Custom|Pause
  (bind _returnvalue (Game|GetPlayerController 0))
  (bind _returnvalue_2 (UserInterface|CreateWidget "/Game/Anthem/Characters/PauseMenu.PauseMenu_C"))
  (bind _output_get (Variables|Default|SetPauseMenu _returnvalue_2))
  (UserInterface|Viewport|AddtoViewport _output_get 0)
  (Input|SetInputModeUIOnly (Game|GetPlayerController 0) _output_get "DoNotLock")
  (Game|SetGamePaused true)
  (bind _output_get_2 (Variables|/Script/Engine.PlayerController|SetbShowMouseCursor _returnvalue true))
  (Variables|/Script/Engine.PlayerController|SetbEnableClickEvents _returnvalue _output_get_2))

(event Custom|UnPause
  (bind _returnvalue (Game|GetPlayerController 0))
  (Widget|RemovefromParent (Variables|Default|GetPauseMenu))
  (Input|SetInputModeGameOnly (Game|GetPlayerController 0))
  (Game|SetGamePaused false)
  (bind _output_get (Variables|/Script/Engine.PlayerController|SetbShowMouseCursor _returnvalue false))
  (Variables|/Script/Engine.PlayerController|SetbEnableClickEvents _returnvalue _output_get))

(event EventBeginPlay)

(event EventTick
  (params (DeltaSeconds :type Float%20%28single-precision%29)))

(fn ConstructionScript)